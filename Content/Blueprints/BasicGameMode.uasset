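; BasicGameMode is a game mode that ramps up difficulty over time and handles game over with a level restart.
; Its tick interval is set in the construction script, and each tick raises the enemy speed multiplier and counts play ticks.
; ReloadLevel disables player input, shows a game over HUD for a short delay, re-enables input, then reopens the current level by name through ResetGame.
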(event Custom|ReloadLevel
  (params (PlayerRef :type Pawn%20Object%20Reference))
  (Input|DisableInput PlayerRef 0)
  (bind _returnvalue (UserInterface|CreateWidget "/Game/Blueprints/HUD/GameOverHUDWidget.GameOverHUDWidget_C"))
  (UserInterface|Viewport|AddtoPlayerScreen _returnvalue)
  (Utilities|FlowControl|Delay 3.0)
  (Widget|RemovefromParent _returnvalue)
  (Input|EnableInput PlayerRef 0)
  (CallFunction|ResetGame))

(event EventBeginPlay)

(event EventTick
  (params (DeltaSeconds :type Float%20%28single-precision%29))
  (Variables|Default|SetStartingEnemySpeedMultiplier (+ (Variables|Default|GetStartingEnemySpeedMultiplier) (Variables|Default|GetEnemySpeedMultiplierIncrements)))
  (Variables|Default|SetPlayTicks (+ (Variables|Default|GetPlayTicks) 1.0)))

(fn ConstructionScript
  (Actor|Tick|SetActorTickInterval (Variables|Default|GetGameTickInterval)))

(fn ResetGame
  (bind _returnvalue (Game|GetCurrentLevelName true))
  (Game|OpenLevel(byName) (Utilities|String|StringToName _returnvalue)))