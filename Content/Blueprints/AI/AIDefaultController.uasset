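; AI controller for AIDefaultCharacter that drives it through the AIDefaultEventGraph behavior tree.
; On possession it caches the character as UFO, and its Run and Walk events forward movement speed changes to that character.
; The behavior tree is run from BeginPlay, possession and every Tick.
; Perception updates for DefaultPlayerPawn write sensing success to CanSeePlayer and reset AISpeedMultiplier on the blackboard.
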(event OnTargetPerceptionUpdated(AIPerception)
  (params (Actor :type Actor%20Object%20Reference) (Stimulus :type AI%20Stimulus%20Structure))
  (bind _returnvalue (AI|GetBlackboard 0))
  (Utilities|Casting|CastToDefaultPlayerPawn Actor)
  (AI|Components|Blackboard|SetValueasBool _returnvalue (Utilities|Name|MakeLiteralName "CanSeePlayer") (.bSuccessfullySensed (Utilities|Struct|BreakAIStimulus Stimulus)))
  (AI|Components|Blackboard|SetValueasFloat _returnvalue (Utilities|Name|MakeLiteralName "AISpeedMultiplier") 1.0))

(event Custom|Run
  ;[1 1 1] Movement speed change assignments
  (Default|Run (Variables|Default|GetUFO)))

(event Custom|Walk
  ;[1 1 1] Movement speed change assignments
  (Default|Walk (Variables|Default|GetUFO)))

(event EventBeginPlay
  ;[1 1 1] Behaviour tree assignment (on begin/process/tick)
  (AI|RunBehaviorTree "/Game/Blueprints/AI/AIDefaultEventGraph.AIDefaultEventGraph"))

(event EventTick
  (params (DeltaSeconds :type Float%20%28single-precision%29))
  ;[1 1 1] Behaviour tree assignment (on begin/process/tick)
  (AI|RunBehaviorTree "/Game/Blueprints/AI/AIDefaultEventGraph.AIDefaultEventGraph"))

(event EventOnPossess
  (params (PossessedPawn :type Pawn%20Object%20Reference))
  ;[1 1 1] Behaviour tree assignment (on begin/process/tick)
  (bind _asaidefault_character (Utilities|Casting|CastToAIDefaultCharacter PossessedPawn))
  (Variables|Default|SetUFO _asaidefault_character)
  (AI|RunBehaviorTree "/Game/Blueprints/AI/AIDefaultEventGraph.AIDefaultEventGraph"))

(fn ConstructionScript)