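; Base AI spawner that keeps a population of BP_AIActorDeefault actors around the player, following a Death, Timer or Wave spawn rule.
; BeginPlay fills the initial count, then Death grows it on a looping timer and Timer periodically tops it up.
; ActorDied replaces each loss under Death, or spawns a larger wave once all die under Wave.
; Spawn points are random navmesh locations, re-rolled until beyond MinimumSpawnRadius from the player.
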(event Custom|ActorDied
  ;[1 1 1] What happens after an actor is killed based on respawn rules
  (Variables|Default|SetNumberOfActors (- (Variables|Default|GetNumberOfActors) 1))
  (switch Utilities|FlowControl|Switch|SwitchonBP_SpawnNewActorsBy (Variables|Default|GetSpawnRule)
    (:NewEnumerator0
      (CallFunction|SpawnNewActor))
    (:NewEnumerator1
      (if (<= (Variables|Default|GetNumberOfActors) 0)
        (for _index (range (Variables|Default|GetNumberOfActors) (Variables|Default|GetMinimumNumberOfActors))
          (CallFunction|SpawnNewActor))
        (CallFunction|IncreaseWaveSize)))))

(event EventBeginPlay
  ;[1 1 1] Setup spawning rules and initially "alive" actors
  (for _index (range (Variables|Default|GetNumberOfActors) (- (Variables|Default|GetMinimumNumberOfActors) 1))
    (CallFunction|SpawnNewActor))
  (switch Utilities|FlowControl|Switch|SwitchonBP_SpawnNewActorsBy (Variables|Default|GetSpawnRule)
    (:NewEnumerator0
      (bind _returnvalue (Utilities|Time|SetTimerbyFunctionName 0 "IncreaseWaveSize" (Variables|Default|GetWaveSizeIncreaseTimer) true))
      (Variables|Default|SetWaveSizeIncreaseHandle _returnvalue))
    (:NewEnumerator3
      (bind _returnvalue_2 (Utilities|Time|SetTimerbyFunctionName 0 "SpawnAdditionalActors" (Variables|Default|GetWaveRespawnTimer) true))
      (Variables|Default|SetWaveRespawnHandle _returnvalue_2))))

(event EventEndPlay
  (params (EndPlayReason :type EEndPlayReason%20Enum :default "Destroyed"))
  ;[1 1 1] Clear all created timer handles
  (Utilities|Time|ClearandInvalidateTimerbyHandle (Variables|Default|GetWaveSizeIncreaseHandle))
  (Utilities|Time|ClearandInvalidateTimerbyHandle (Variables|Default|GetWaveRespawnHandle)))

(fn ConstructionScript
  (bind _asbp_basic_game_mode (Utilities|Casting|CastToBP_BasicGameMode (Game|GetGameMode)))
  (Variables|Default|SetGameMode _asbp_basic_game_mode))

(fn GetRandomSpawnLocation
  (LocalVariables|SetSpawnRadius (+ (Variables|Default|GetMinimumSpawnRadius) 1e+03))
  (LocalVariables|SetPlayerLocation (Transformation|GetActorLocation (Game|Player|GetPlayerPawn 0)))
  ;[1 1 1] Find actor spawn location at least @SpawnRadius units away from player
  (LocalVariables|SetResult (Math|Vector|MakeVector (.x (.RandomLocation (Class|NavigationSystemV1|GetRandomPointinNavigableRadius (LocalVariables|GetPlayerLocation) (LocalVariables|GetSpawnRadius) 0 0))) (.y (.RandomLocation (Class|NavigationSystemV1|GetRandomPointinNavigableRadius (LocalVariables|GetPlayerLocation) (LocalVariables|GetSpawnRadius) 0 0))) 1e+02))
  (while (<= (Utilities|CalculateVectorDistance (LocalVariables|GetPlayerLocation) (LocalVariables|GetResult)) (Variables|Default|GetMinimumSpawnRadius))
    (LocalVariables|SetResult (Math|Vector|MakeVector (.x (.RandomLocation (Class|NavigationSystemV1|GetRandomPointinNavigableRadius (LocalVariables|GetPlayerLocation) (LocalVariables|GetSpawnRadius) 0 0))) (.y (.RandomLocation (Class|NavigationSystemV1|GetRandomPointinNavigableRadius (LocalVariables|GetPlayerLocation) (LocalVariables|GetSpawnRadius) 0 0))) 1e+02)))
  (return (LocalVariables|GetResult)))

(fn SpawnNewActor
  (bind _randomvector (CallFunction|GetRandomSpawnLocation))
  (Game|SpawnActorfromClass "/Game/Blueprints/AI/BP_AIActorDeefault.BP_AIActorDeefault_C" (Math|Transform|MakeTransform _randomvector "0, 0, 0" "1.000000,1.000000,1.000000") "AdjustIfPossibleButAlwaysSpawn" 0 2.0 1e+03 4e+01 1.0 0)
  (Math|Integer|IncrementInt (Variables|Default|GetNumberOfActors)))

(fn IncreaseWaveSize
  (Math|Integer|IncrementInt (Variables|Default|GetMinimumNumberOfActors)
    (:%20%20
      (switch Utilities|FlowControl|Switch|SwitchonBP_SpawnNewActorsBy (Variables|Default|GetSpawnRule)
        (:NewEnumerator0
          (CallFunction|SpawnNewActor))))))

(fn SpawnAdditionalActors
  (for _index (range (Variables|Default|GetNumberOfActors) (- (Variables|Default|GetMinimumNumberOfActors) 1))
    (CallFunction|SpawnNewActor)))