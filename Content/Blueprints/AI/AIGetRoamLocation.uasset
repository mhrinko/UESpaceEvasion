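; Behavior tree task that picks a random navigable roam location within a fixed radius around the AI.
; If the moving flag is not already set, it sets it, calls Walk on the AIDefaultController and writes the point to the blackboard with a fixed height.
; Both paths finish with the success result of a random navigable point query, so an already moving AI keeps its stored location.
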(event EventReceiveExecute
  (params (OwnerActor :type Actor%20Object%20Reference))
  (bind _returnvalue (Transformation|GetActorLocation OwnerActor))
  (bind _bismoving (Variables|Default|GetbIsMoving))
  (bind (_randomlocation _returnvalue_2) (Class|NavigationSystemV1|GetRandomPointinNavigableRadius _returnvalue 5e+03 0 0))
  (bind (_x _y) (Math|Vector|BreakVector _randomlocation))
  (if (Class|BTFunctionLibrary|GetBlackboardValueasBool _bismoving)
    _
    (else
      (Class|BTFunctionLibrary|SetBlackboardValueasBool _bismoving true)
      (bind _asaidefault_controller (Utilities|Casting|CastToAIDefaultController OwnerActor))
      (Default|Walk _asaidefault_controller)
      (AI|BehaviorTree|SetBlackboardValueasVector (Variables|Default|GetRandomLocationKey) (Math|Vector|MakeVector _x _y 1e+02))))
  (AI|BehaviorTree|FinishExecute _returnvalue_2))