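; Base enemy AI actor that wanders between random destinations and chases the player when AI perception senses them.
; Movement is a manual swept lerp facing the target, scaled by the game mode's speed multiplier and a perception-driven boost, repicking destinations when blocked.
; Mesh overlap deals damage immediately and on a looping timer.
; It links itself to a health bar widget, and death notifies the game mode's spawner before destroying the actor.
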(event OnTargetPerceptionUpdated(AIPerception)
  (params (Actor :type Actor%20Object%20Reference) (Stimulus :type AI%20Stimulus%20Structure))
  (bind _returnvalue (Game|Player|GetPlayerPawn 0))
  ;[1 1 1] Switch slow and fast speeds when player is out of range and in range respectively
  (if (and (== Actor _returnvalue) (.bSuccessfullySensed (Utilities|Struct|BreakAIStimulus Stimulus)))
    (Variables|AIControls|SetbCanSeePlayer true)
    (Variables|Default|SetTargetPlayerPawn _returnvalue)
    (Variables|PublicStats|SetSpeedMultiplier (* (Variables|PublicStats|GetSpeedMultiplier) (Variables|Default|GetDefaultSpeedUp)))
    (else
      (Variables|AIControls|SetbCanSeePlayer false)
      (Variables|PublicStats|SetSpeedMultiplier (/ (Variables|PublicStats|GetSpeedMultiplier) (Variables|Default|GetDefaultSpeedUp))))))

(event OnComponentBeginOverlap(EnemyMesh)
  (params (OverlappedComponent :type Primitive%20Component%20Object%20Reference) (OtherActor :type Actor%20Object%20Reference) (OtherComp :type Primitive%20Component%20Object%20Reference) (OtherBodyIndex :type Integer) (bFromSweep :type Boolean) (SweepResult :type Hit%20Result%20Structure%20%28by%20ref%29))
  (Variables|Default|SetIsOverlapping true)
  (Variables|Default|SetOverlappedActor OtherActor)
  (CallFunction|ApplyDamageonCollision)
  (bind _returnvalue (Utilities|Time|SetTimerbyFunctionName 0 "ApplyDamageOnCollision" (Variables|PublicStats|GetCollisionDamageTimer) true))
  (Variables|Default|SetDamageTimerHandle _returnvalue))

(event OnComponentEndOverlap(EnemyMesh)
  (params (OverlappedComponent :type Primitive%20Component%20Object%20Reference) (OtherActor :type Actor%20Object%20Reference) (OtherComp :type Primitive%20Component%20Object%20Reference) (OtherBodyIndex :type Integer))
  (Variables|Default|SetIsOverlapping false)
  (Utilities|Time|ClearandInvalidateTimerbyHandle (Variables|Default|GetDamageTimerHandle)))

(event EventTick
  (params (DeltaSeconds :type Float%20%28single-precision%29))
  (Variables|Default|SetDeltaSeconds DeltaSeconds)
  (if (Variables|AIControls|GetbCanSeePlayer)
    ;[1 1 1] Move to player, if it's in the vision radius
    (Movement|MovetoPawn (Variables|Default|GetTargetPlayerPawn) (Variables|Default|GetDeltaSeconds))
    (else
      ;[1 1 1] Move to random direction
      (if (<= (Math|Vector|VectorLength (- (Variables|AIControls|GetMovementDirection) (Transformation|GetActorLocation))) (Variables|PublicStats|GetDirectionResetDistance))
        (bind _randomvector (Utility|GetRandomDirection))
        (Variables|AIControls|SetMovementDirection _randomvector))
      (Movement|MovetoLocation (Variables|AIControls|GetMovementDirection) (Variables|Default|GetDeltaSeconds)))))

(event EventBeginPlay
  (bind _self self)
  ;[1 1 1] Get game mode to keep track of movement acceleration over time, add reference to widget component
  (bind _asbasic_game_mode (Utilities|Casting|CastToBasicGameMode (Game|GetGameMode)))
  (Variables|Default|SetbpGameMode _asbasic_game_mode)
  (bind _asbp_aihealth_bar (Utilities|Casting|CastToBP_AIHealthBar (UserInterface|GetUserWidgetObject (Variables|Default|GetHealthWidget)))
    (:then
      (Variables|/Game/Blueprints/AI/BP_AIHealthBar.BP_AIHealthBar_C|SetActorAI _asbp_aihealth_bar _self))
    (:CastFailed
      (Development|PrintString (Utilities|String|Append (Utilities|GetDisplayName _self) "failed to assign actor ref to its widget component")))))

(event Game|Damage|EventAnyDamage
  (params (Damage :type Float%20%28single-precision%29) (DamageType :type Damage%20Type%20Object%20Reference) (InstigatedBy :type Controller%20Object%20Reference) (DamageCauser :type Actor%20Object%20Reference))
  (bind _output_get (Variables|Default|SetHealth (- (Variables|Default|GetHealth) Damage)))
  (if (<= _output_get 0.0)
    (Default|ActorDied (Variables|/Game/Blueprints/BasicGameMode.BasicGameMode_C|GetSpawner (Variables|Default|GetbpGameMode)))
    (Actor|DestroyActor)))

(fn ConstructionScript
  (Variables|Default|SetHealth (Variables|PublicStats|GetMaxHealth))
  (bind _randomvector (Utility|GetRandomDirection))
  (Variables|AIControls|SetMovementDirection _randomvector))

(fn GetRandomDirection
  (return (Utilities|GetRandomLication)))

(fn MovetoLocation
  (params (Destination :type Vector) (DeltaSeconds :type Float%20%28single-precision%29))
  (bind _returnvalue (Transformation|GetActorLocation))
  ;[1 1 1] Calculating and setting new location and rotation
  (bind _output_get (LocalVariables|SetLocalDestiation Destination))
  (LocalVariables|SetLocalDistance (Utilities|CalculateVectorDistance _returnvalue (LocalVariables|GetLocalDestiation)))
  (Transformation|SetActorRotation (Math|Rotator|FindLookatRotation _returnvalue (LocalVariables|GetLocalDestiation)))
  ;[1 1 1] As if reached destination
  (if (<= (LocalVariables|GetLocalDistance) 2.0)
    ;[1 1 1] Find new destination if collision happens
    (bind _randomvector (Utility|GetRandomDirection :!label _label))
    (Variables|AIControls|SetMovementDirection _randomvector)
    (else
      (bind _sweephitresult (Transformation|SetActorRelativeLocation (Math|Vector|Lerp(Vector) _returnvalue _output_get (* (/ DeltaSeconds (/ (LocalVariables|GetLocalDistance) (Variables|PublicStats|GetSpeed))) (Variables|PublicStats|GetSpeedMultiplier) (Variables|/Game/Blueprints/BasicGameMode.BasicGameMode_C|GetStartingEnemySpeedMultiplier (Variables|Default|GetbpGameMode)))) true))
      (if (.bBlockingHit (Collision|BreakHitResult _sweephitresult))
        (goto _label)))))

(fn MovetoPawn
  (params (DestinationPawn :type Pawn%20Object%20Reference) (DeltaSeconds :type Float%20%28single-precision%29))
  (Movement|MovetoLocation (Transformation|GetActorLocation DestinationPawn) DeltaSeconds))

(fn ApplyDamageonCollision
  (if (Variables|Default|GetIsOverlapping)
    (Game|Damage|ApplyDamage (Variables|Default|GetOverlappedActor) (Variables|PublicStats|GetCollisionDamageDealt) 0 0)))