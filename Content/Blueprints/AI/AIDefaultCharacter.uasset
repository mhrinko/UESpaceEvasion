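; AIDefaultCharacter is an AI character with Run and Walk events whose speeds scale with a global multiplier.
; On BeginPlay and every Tick it copies AISpeedMultiplier from BasicGameMode into its blackboard.
; Run and Walk read that blackboard value to scale a fixed base MaxWalkSpeed, so a changed multiplier affects movement only when either event next fires.
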(event Custom|Run
  (Variables|/Script/Engine.CharacterMovementComponent|SetMaxWalkSpeed (Variables|Character|GetCharacterMovement) (* 4e+02 (Class|BlackboardComponent|GetValueasFloat (Variables|Default|GetCurrentBlackboard) (Variables|Default|GetKeyAISpeedMultiplier)))))

(event Custom|Walk
  (Variables|/Script/Engine.CharacterMovementComponent|SetMaxWalkSpeed (Variables|Character|GetCharacterMovement) (* 2e+02 (Class|BlackboardComponent|GetValueasFloat (Variables|Default|GetCurrentBlackboard) (Variables|Default|GetKeyAISpeedMultiplier)))))

(event EventBeginPlay
  (bind _asbasic_game_mode (Utilities|Casting|CastToBasicGameMode (Game|GetGameMode)))
  (bind _output_get (Variables|Default|SetKeyAISpeedMultiplier (Utilities|Name|MakeLiteralName "AISpeedMultiplier")))
  (bind _output_get_2 (Variables|Default|SetCurrentBlackboard (AI|GetBlackboard 0)))
  (AI|Components|Blackboard|SetValueasFloat _output_get_2 _output_get (Variables|/Game/Blueprints/BasicGameMode.BasicGameMode_C|GetAISpeedMultiplier _asbasic_game_mode)))

(event EventTick
  (params (DeltaSeconds :type Float%20%28single-precision%29))
  (bind _asbasic_game_mode (Utilities|Casting|CastToBasicGameMode (Game|GetGameMode)))
  (AI|Components|Blackboard|SetValueasFloat (Variables|Default|GetCurrentBlackboard) (Variables|Default|GetKeyAISpeedMultiplier) (Variables|/Game/Blueprints/BasicGameMode.BasicGameMode_C|GetAISpeedMultiplier _asbasic_game_mode)))

(fn ConstructionScript)