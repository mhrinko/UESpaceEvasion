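; Game mode that runs an enemy-spawning score game, tracking player score and an enemy speed multiplier that rises during play.
; On BeginPlay it spawns and configures BP_SpawnerBase.
; Speed rises either on a custom-interval tick or through the SpeedUp event, with SpeedUpEveryWave disabling the tick ramp.
; Death disables input and shows a game-over widget for a short delay before reopening the current level, while ReloadLevel reopens it immediately.
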(event Custom|ReloadLevel
  (params (PlayerRef :type Pawn%20Object%20Reference))
  (CallFunction|ResetGame))

(event Custom|DeathReloadLevel
  (params (PlayerRef :type Pawn%20Object%20Reference))
  (Input|DisableInput PlayerRef 0)
  (bind _returnvalue (UserInterface|CreateWidget "/Game/Blueprints/HUD/BP_GameOverWidgetHUD.BP_GameOverWidgetHUD_C"))
  (UserInterface|Viewport|AddtoPlayerScreen _returnvalue)
  (Utilities|FlowControl|Delay 3.0)
  (Widget|RemovefromParent _returnvalue)
  (Input|EnableInput PlayerRef 0)
  (CallFunction|ResetGame))

(event Custom|PlayerScoreIncreased
  (params (Increment :type Integer))
  (Variables|Default|SetPlayerScore (+ Increment (Variables|Default|GetPlayerScore))))

(event Custom|SpeedUp
  (Variables|Default|SetStartingEnemySpeedMultiplier (+ (Variables|Default|GetStartingEnemySpeedMultiplier) (* (Variables|Default|GetEnemySpeedMultiplierIncrements) 1.0))))

(event EventBeginPlay
  ;[1 1 1] Setup spawner
  (bind _returnvalue (Game|SpawnActorfromClass "/Game/Blueprints/AI/Spawner/BP_SpawnerBase.BP_SpawnerBase_C" (|EmptyTransform) "AlwaysSpawn" 0 "NewEnumerator1" 4 1e+03 2e+01 2e+01 (Variables|Default|GetEnemyDiesOnImpact) (not (Variables|Default|GetSpeedUpEveryWave)) 0))
  (Variables|Default|SetSpawner _returnvalue))

(event EventTick
  (params (DeltaSeconds :type Float%20%28single-precision%29))
  (if (not (Variables|Default|GetSpeedUpEveryWave))
    (Variables|Default|SetStartingEnemySpeedMultiplier (+ (Variables|Default|GetStartingEnemySpeedMultiplier) (Variables|Default|GetEnemySpeedMultiplierIncrements)))
    (Variables|Default|SetPlayTicks (+ (Variables|Default|GetPlayTicks) 1.0))))

(fn ConstructionScript
  (Actor|Tick|SetActorTickInterval (Variables|Default|GetGameTickInterval)))

(fn ResetGame
  (bind _returnvalue (Game|GetCurrentLevelName true))
  (Game|OpenLevel(byName) (Utilities|String|StringToName _returnvalue)))

(fn GetPlayerScoreText
  (return (Utilities|Text|ToText(Integer) (Variables|Default|GetPlayerScore))))